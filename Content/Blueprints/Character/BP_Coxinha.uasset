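; Player character with camera-relative movement, a directional dash, toggleable slow motion and automatic twin-barrel fire.
; Dash polls WASD and launches along the mesh's forward or right axes after a short DoOnce-guarded delay.
; Slow motion flip-flops global time dilation, setting camera post-process only when enabled.
; Holding Fire runs a looping timer that spawns projectiles, muzzle flashes and gunshot sounds from two arrows.
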(event `InputAction|Slow Motion`
  (params (Key :type "Key Structure"))
  (:`Pressed`
    (`/Engine/EditorBlueprintResources/StandardMacros.FlipFlop`
      (:`A`
        (set `CameraComponent.PostProcessSettings` (make `PostProcessSettings`) (`self.Camera`))
        (`GameplayStatics.SetGlobalTimeDilation` 0.2))
      (:`B`
        (`GameplayStatics.SetGlobalTimeDilation` 1.0)))))

(event `InputAction|Dash`
  (params (Key :type "Key Structure"))
  ;[0.004949 0.01923 1] Dash
  (:`Pressed`
    (if (`PlayerController.IsInputKeyDown` (`GameplayStatics.GetPlayerController` 0) "W")
      (`/Engine/EditorBlueprintResources/StandardMacros.DoOnce` false :!label _label
        (:`Completed`
          (`KismetSystemLibrary.Delay` 0.05)
          (`self.LaunchCharacter` (* (`SceneComponent.GetForwardVector` (`self.Mesh`)) 4000.0))
          (goto _label :!via `Reset`)))
      (elif (`PlayerController.IsInputKeyDown` (`GameplayStatics.GetPlayerController` 0) "S")
        (`/Engine/EditorBlueprintResources/StandardMacros.DoOnce` false :!label _label_2
          (:`Completed`
            (`KismetSystemLibrary.Delay` 0.05)
            (`self.LaunchCharacter` (* (`SceneComponent.GetForwardVector` (`self.Mesh`)) -4000.0))
            (goto _label_2 :!via `Reset`)))
        (elif (`PlayerController.IsInputKeyDown` (`GameplayStatics.GetPlayerController` 0) "A")
          (`/Engine/EditorBlueprintResources/StandardMacros.DoOnce` false :!label _label_3
            (:`Completed`
              (`KismetSystemLibrary.Delay` 0.05)
              (`self.LaunchCharacter` (* (`SceneComponent.GetRightVector` (`self.Mesh`)) -4000.0))
              (goto _label_3 :!via `Reset`)))
          (elif (`PlayerController.IsInputKeyDown` (`GameplayStatics.GetPlayerController` 0) "D")
            (`/Engine/EditorBlueprintResources/StandardMacros.DoOnce` false :!label _label_4
              (:`Completed`
                (`KismetSystemLibrary.Delay` 0.05)
                (`self.LaunchCharacter` (* (`SceneComponent.GetRightVector` (`self.Mesh`)) 4000.0))
                (goto _label_4 :!via `Reset`)))))))))

(event `InputAxis|ForwardBackward`
  (params (AxisValue :type "Float (single-precision)"))
  ;[0.01576 1 0] Input Movement
  (`self.AddMovementInput` (`KismetMathLibrary.GetForwardVector` (`KismetMathLibrary.MakeRotator` 0.0 0.0 (.yaw (`self.GetControlRotation`)))) AxisValue))

(event `InputAxis|LeftRight`
  (params (AxisValue :type "Float (single-precision)"))
  ;[0.01576 1 0] Input Movement
  (`self.AddMovementInput` (`KismetMathLibrary.GetRightVector` (`KismetMathLibrary.MakeRotator` 0.0 0.0 (.yaw (`self.GetControlRotation`)))) AxisValue))

(event `InputAxis|Turn`
  (params (AxisValue :type "Float (single-precision)"))
  ;[0.01576 1 0] Input Movement
  (`self.AddMovementInput` (`KismetMathLibrary.GetForwardVector` (`self.GetControlRotation`)) AxisValue)
  (`self.AddControllerYawInput` AxisValue))

(event `InputAction|Fire`
  (params (Key :type "Key Structure"))
  (:`Pressed`
    (bind _returnvalue (`KismetSystemLibrary.K2_SetTimerDelegate` (delegate `AutoFire`) 0.25 true)))
  (:`Released`
    (`KismetSystemLibrary.K2_ClearAndInvalidateTimerHandle` _returnvalue)))

(event `AutoFire`
  (`|ExecutionSequence`
    (:`then_0`
      (`ActorComponent.Activate` (`self.NS_AR_Muzzleflash_1_ONCE`) false)
      (`GameplayStatics.PlaySoundAtLocation` "/Game/Sound/8d82b5_M4A1_Firing_Sound_Effect_Cue.8d82b5_M4A1_Firing_Sound_Effect_Cue" (0.0 0.0 0.0) (struct) 1.0 0.9 0.0 null null null)
      (`|SpawnActorFromClass` "/Game/Projectile/AR4Projectile.AR4Projectile_C" (`SceneComponent.K2_GetComponentToWorld` (`self.Arrow2`)) "Undefined" "OverrideRootScale" (`self.Selfref`) null))
    (:`then_1`
      (`ActorComponent.Activate` (`self.NS_AR_Muzzleflash_1_ONCE1`) false)
      (`GameplayStatics.PlaySoundAtLocation` "/Game/Sound/8d82b5_M4A1_Firing_Sound_Effect_Cue.8d82b5_M4A1_Firing_Sound_Effect_Cue" (0.0 0.0 0.0) (struct) 1.0 0.9 0.0 null null null)
      (`|SpawnActorFromClass` "/Game/Projectile/AR4Projectile.AR4Projectile_C" (`SceneComponent.K2_GetComponentToWorld` (`self.Arrow1`)) "Undefined" "OverrideRootScale" (`self.Selfref`) null))))

(fn `UserConstructionScript`)