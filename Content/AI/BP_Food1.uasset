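; BP_Food1 is an AI-folder actor with a capsule component that takes projectile damage and can be destroyed.
; On a capsule hit by a BaseProjectile, it subtracts the projectile's Damage directly from MaxHealth, which doubles as current health.
; It prints the remaining value and destroys itself at zero or below.
; The graphs contain no movement or decision logic.
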(event `self.CapsuleComponent.OnComponentHit`
  (params (HitComponent :type "PrimitiveComponent Object Reference") (OtherActor :type "Actor Object Reference") (OtherComp :type "PrimitiveComponent Object Reference") (NormalImpulse :type "Vector Structure") (Hit :type "HitResult Structure (by ref)"))
  (bind _asbase_projectile (cast `/Game/Projectile/BaseProjectile` OtherActor))
  (bind _output_get (set `self.MaxHealth` (- (`self.MaxHealth`) (`/Game/Projectile/BaseProjectile.Damage` _asbase_projectile))))
  (`KismetSystemLibrary.PrintString` (`KismetStringLibrary.Conv_IntToString` _output_get))
  (if (<= (`self.MaxHealth`) 0)
    (`self.K2_DestroyActor`)))

(fn `UserConstructionScript`
  (`parent.UserConstructionScript`))