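; BP_AiSpawn is a spawner that places BP_Food1 actors in the level when play begins.
; BeginPlay calls SpawnAi ActorsAmount times, each picking a random point around the bounds origin of the SpawnRadious component.
; The sampling box uses that component's Z extent on all three axes, and yaw comes from an unscaled RandomFloat, so rotation varies by at most one degree.
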(event `self.ReceiveBeginPlay`
  (for _ (range 1 (+ (`self.ActorsAmount`) 1))
    (`self.SpawnAi`)))

(fn `SpawnAi`
  (bind (_origin _boxextent) (`KismetSystemLibrary.GetComponentBounds` (`self.SpawnRadious`)))
  (`|SpawnActorFromClass` "/Game/AI/BP_Food1.BP_Food1_C" (`KismetMathLibrary.MakeTransform` (`KismetMathLibrary.RandomPointInBoundingBox` _origin (`KismetMathLibrary.Conv_DoubleToVector` (.z _boxextent))) (`KismetMathLibrary.MakeRotator` 0.0 0.0 (`KismetMathLibrary.RandomFloat`))) "Undefined" "OverrideRootScale" null null))

(fn `UserConstructionScript`)